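; BP_Fur is an actor that renders fur on a chosen mesh using stacked mesh layers, a shell-style technique.
; The construction script applies the mesh to the base component, then adds a copy per fur layer.
; Each copy gets a dynamic material instance receiving its layer index, layer count and velocity.
; Tick stores the actor's velocity, but only the construction script passes it to the materials.
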(event EventTick
  (params (DeltaSeconds :type Float%20%28single-precision%29))
  (Variables|Default|SetVelocity (Transformation|GetVelocity self)))

(fn ConstructionScript
  ;[0.15 0.15 0.15 0.5] Replace the 'StaticMesh' with a mesh of our choice
  (Components|StaticMesh|SetStaticMesh (Variables|Default|GetStaticMesh) (Variables|Default|GetMesh))
  ;[0.15 0.15 0.15 0.5] Add copies of the mesh that will act as each individual layer of fur.
  (for _index (range 0 (Variables|Default|GetFurLayers))
    (bind _returnvalue (AddComponent|AddStaticMeshComponent false))
    (Components|StaticMesh|SetStaticMesh _returnvalue (Variables|Default|GetMesh))
    ;[0.15 0.15 0.15 0.5] Create a material instance for each fur layer and setting the required parameters
    (bind _returnvalue_2 (Rendering|Material|CreateDynamicMaterialInstance _returnvalue 0 (Variables|Default|GetMaterial) "None" :!class /Script/Engine.PrimitiveComponent))
    (Rendering|Material|SetScalarParameterValue _returnvalue_2 "Layer Index" (Math|Conversions|ToFloat(Integer) _index) :!class /Script/Engine.MaterialInstanceDynamic)
    (Rendering|Material|SetScalarParameterValue _returnvalue_2 "Layer Count" (Math|Conversions|ToFloat(Integer) (Variables|Default|GetFurLayers)) :!class /Script/Engine.MaterialInstanceDynamic)
    (Rendering|Material|SetVectorParameterValue _returnvalue_2 "Velocity" (Math|Conversions|ToLinearColor(Vector) (Variables|Default|GetVelocity)) :!class /Script/Engine.MaterialInstanceDynamic)))